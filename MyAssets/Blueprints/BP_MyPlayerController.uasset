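; Player controller that tracks gold, mana and health, pushes them to the HUD, and handles spell casting.
; BeginPlay creates the HUD and hidden spellbook and initializes the stats; M toggles the spellbook.
; SpellLaunch checks magic permission, menu state, availability and mana, then plays animation and particles, with special handling for teleportation.
; Input fires rebindable single-listener dispatchers for interact, cast and TPS/FPS camera switching.
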(event `GoldOnStart`
  ;[1 1 1] Gold Related
  (bind _output_get (set `self.CurrentGold` 5000))
  (`/Game/MyAssets/Blueprints/UI/WBP_MyUI.GoldUpdate` (`self.MyUI`) (`KismetTextLibrary.Conv_IntToText` _output_get)))

(event `Init_Shop`
  ;[1 1 1] Spell Shop Related
  (bind _returnvalue (`|CreateWidget` "/Game/MyAssets/Blueprints/UI/WBP_Shop.WBP_Shop_C"))
  (bind _output_get (set `self.My Shop` _returnvalue))
  (`UserWidget.AddToViewport` _output_get 0)
  (`Widget.SetVisibility` _output_get "Hidden"))

(event `DecreaseGold`
  (params (`Nb Subtracted` :type Integer))
  ;[1 1 1] Gold Related
  (bind _output_get (set `self.CurrentGold` (- (`self.CurrentGold`) `Nb Subtracted`)))
  (`/Game/MyAssets/Blueprints/UI/WBP_MyUI.GoldUpdate` (`self.MyUI`) (`KismetTextLibrary.Conv_IntToText` _output_get)))

(event `IncreaseGold`
  (params (`Nb Added` :type Integer))
  ;[1 1 1] Gold Related
  (bind _output_get (set `self.CurrentGold` (+ (`self.CurrentGold`) `Nb Added`)))
  (`/Game/MyAssets/Blueprints/UI/WBP_MyUI.GoldUpdate` (`self.MyUI`) (`KismetTextLibrary.Conv_IntToText` _output_get)))

(event `Display Shop`
  ;[1 1 1] Spell Shop Related
  (`Widget.SetVisibility` (`self.My Shop`) "Visible")
  (set `self.bShowMouseCursor` true)
  (set `self.MenuOpened` true))

(event `InitSpellBook`
  ;[1 1 1] SpellBook
  (bind _returnvalue (`|CreateWidget` "/Game/MyAssets/Blueprints/UI/WBP_SpellBook.WBP_SpellBook_C"))
  (bind _output_get (set `self.MySpellBook` _returnvalue))
  (`UserWidget.AddToViewport` _output_get 0)
  (`Widget.SetVisibility` _output_get "Hidden"))

(event `HideShop`
  ;[1 1 1] Spell Shop Related
  (`Widget.SetVisibility` (`self.My Shop`) "Hidden")
  (set `self.bShowMouseCursor` false)
  (set `self.MenuOpened` false))

(event `Key|M`
  (params (Key :type "Key Structure"))
  (bind _myspellbook (`self.MySpellBook`))
  ;[1 1 1] SpellBook
  (:`Pressed`
    (`/Engine/EditorBlueprintResources/StandardMacros.FlipFlop`
      (:`A`
        (`Widget.SetVisibility` _myspellbook "Visible")
        (set `self.bShowMouseCursor` true)
        (set `self.MenuOpened` true))
      (:`B`
        (`Widget.SetVisibility` _myspellbook "Hidden")
        (set `self.bShowMouseCursor` false)
        (set `self.MenuOpened` false)))))

(event `ManaOnStart`
  ;[1 1 1] Mana Related
  (bind _output_get (set `self.CurrentMana` (`self.MaxMana`)))
  (`/Game/MyAssets/Blueprints/UI/WBP_MyUI.ManaUpdate` (`self.MyUI`) (`KismetTextLibrary.Conv_IntToText` _output_get)))

(event `DecreaseMana`
  (params (`Nb Substracted` :type Integer))
  ;[1 1 1] Mana Related
  (bind _output_get (set `self.CurrentMana` (- (`self.CurrentMana`) `Nb Substracted`)))
  (`/Game/MyAssets/Blueprints/UI/WBP_MyUI.ManaUpdate` (`self.MyUI`) (`KismetTextLibrary.Conv_IntToText` _output_get)))

(event `IncreaseMana`
  (params (`Nb Added` :type Integer))
  ;[1 1 1] Mana Related
  (bind _output_get (set `self.CurrentMana` (+ (`self.CurrentMana`) `Nb Added`)))
  (`/Game/MyAssets/Blueprints/UI/WBP_MyUI.ManaUpdate` (`self.MyUI`) (`KismetTextLibrary.Conv_IntToText` _output_get)))

(event `DisplayCurrentSpell`
  (`/Game/MyAssets/Blueprints/UI/WBP_MyUI.SpellUpdate` (`self.MyUI`) (`KismetTextLibrary.Conv_StringToText` (`/Game/MyAssets/Blueprints/DataAssets/DA_Spell.Name` (`self.EquipedSpell`)))))

(event `self.ReceiveBeginPlay`
  (bind _returnvalue (`|CreateWidget` "/Game/MyAssets/Blueprints/UI/WBP_MyUI.WBP_MyUI_C"))
  (bind _output_get (set `self.MyUI` _returnvalue))
  (`UserWidget.AddToViewport` _output_get 0)
  (`self.LifeOnStart`)
  (`self.ManaOnStart`)
  (`self.GoldOnStart`)
  (`self.InitSpellBook`)
  (`self.Init_Shop`))

(event `LifeOnStart`
  ;[1 1 1] Life Related
  (bind _output_get (set `self.CurrentLife` (`self.MaxLife`)))
  (`/Game/MyAssets/Blueprints/UI/WBP_MyUI.HealthUpdate` (`self.MyUI`) (`KismetTextLibrary.Conv_IntToText` _output_get)))

(event `InputAction|Interaction`
  (params (Key :type "Key Structure"))
  ;[1 1 1] The Binding of Mes Touches
  (:`Pressed`
    (`self.OnE`)))

(event `DecreaseHealth`
  (params (NbSubstracted :type Integer :default 20))
  ;[1 1 1] Life Related
  (bind _output_get (set `self.CurrentLife` (- (`self.CurrentLife`) NbSubstracted)))
  (`/Game/MyAssets/Blueprints/UI/WBP_MyUI.HealthUpdate` (`self.MyUI`) (`KismetTextLibrary.Conv_IntToText` _output_get)))

(event `IncreaseHealth`
  (params (NbAdded :type Integer :default 20))
  ;[1 1 1] Life Related
  (bind _output_get (set `self.CurrentLife` (+ NbAdded (`self.CurrentLife`))))
  (`/Game/MyAssets/Blueprints/UI/WBP_MyUI.HealthUpdate` (`self.MyUI`) (`KismetTextLibrary.Conv_IntToText` _output_get)))

(event `InputAction|Spell_Throw`
  (params (Key :type "Key Structure"))
  ;[1 1 1] The Binding of Mes Touches
  (:`Pressed`
    (`self.OnLeftClick`)))

(event `SpellLaunch`
  (if (`self.CanDoMagic`)
    (if (`self.MenuOpened`)
      _
      (elif (`/Game/MyAssets/Blueprints/DataAssets/DA_Spell.Available` (`self.EquipedSpell`))
        (`/Engine/EditorBlueprintResources/StandardMacros.CompareInt` (`/Game/MyAssets/Blueprints/DataAssets/DA_Spell.ManaCost` (`self.EquipedSpell`)) (`self.CurrentMana`)
          (:`==`
            _)
          (:`<`
            _))
        (if true
          (`KismetSystemLibrary.PrintString` (`/Game/MyAssets/Blueprints/DataAssets/DA_Spell.Name` (`self.EquipedSpell`)))
          (`self.DecreaseMana` (`/Game/MyAssets/Blueprints/DataAssets/DA_Spell.ManaCost` (`self.EquipedSpell`)))
          (`self.NewSpell`)
          (bind _asthird_person_character (cast `/Game/ThirdPersonBP/Blueprints/ThirdPersonCharacter` (`GameplayStatics.GetPlayerCharacter` 0)))
          (`self.PlayAnimation` (`/Game/MyAssets/Blueprints/DataAssets/DA_Spell.AnimationToPlay` (`self.EquipedSpell`)))
          (if (`KismetSystemLibrary.IsValid` (`self.EquipedSpell`))
            (bind _returnvalue (`GameplayStatics.SpawnEmitterAtLocation` (`/Game/MyAssets/Blueprints/DataAssets/DA_Spell.ParticleSpawned` (`self.EquipedSpell`)) (`SceneComponent.K2_GetComponentLocation` (`/Game/ThirdPersonBP/Blueprints/ThirdPersonCharacter.SpellSpawner` _asthird_person_character))))
            (`KismetSystemLibrary.Delay` 3.0)
            (`ActorComponent.K2_DestroyComponent` _returnvalue)
            (else
              (`KismetSystemLibrary.PrintString` "Press M to select a spell"))))
        (else
          (`KismetSystemLibrary.PrintString` "You don't have this spell."))))
    (else
      (`KismetSystemLibrary.PrintString` "Please go to the training ground to practice magic"))))

(event `InputAction|View_Switch`
  (params (Key :type "Key Structure"))
  ;[1 1 1] The Binding of Mes Touches
  (:`Pressed`
    (`self.OnTab`)))

(event `PlayAnimation`
  (params (NewAnimToPlay :type "AnimationAsset Object Reference"))
  (bind _asthird_person_character (cast `/Game/ThirdPersonBP/Blueprints/ThirdPersonCharacter` (`GameplayStatics.GetPlayerCharacter` 0)))
  (`SkeletalMeshComponent.PlayAnimation` (`Character.Mesh` _asthird_person_character) NewAnimToPlay false)
  (`KismetSystemLibrary.Delay` 1.0)
  (`SkeletalMeshComponent.SetAnimationMode` (`Character.Mesh` (`GameplayStatics.GetPlayerCharacter` 0)) "AnimationBlueprint"))

(event `Switch View`
  ;[1 1 1] Switch TPS / FPS Cam
  (`/Engine/EditorBlueprintResources/StandardMacros.FlipFlop`
    (:`A`
      (bind _asthird_person_character (cast `/Game/ThirdPersonBP/Blueprints/ThirdPersonCharacter` (`GameplayStatics.GetPlayerCharacter` 0)))
      (`SceneComponent.K2_SetRelativeLocation` (`/Game/ThirdPersonBP/Blueprints/ThirdPersonCharacter.FollowCamera` _asthird_person_character) (`/Game/ThirdPersonBP/Blueprints/ThirdPersonCharacter.FPSCam` _asthird_person_character) false false)
      (`KismetSystemLibrary.PrintString` "FPS View"))
    (:`B`
      (bind _asthird_person_character_2 (cast `/Game/ThirdPersonBP/Blueprints/ThirdPersonCharacter` (`GameplayStatics.GetPlayerCharacter` 0)))
      (`SceneComponent.K2_SetRelativeLocation` (`/Game/ThirdPersonBP/Blueprints/ThirdPersonCharacter.FollowCamera` _asthird_person_character_2) (`/Game/ThirdPersonBP/Blueprints/ThirdPersonCharacter.TPSCam` _asthird_person_character_2) false false)
      (`KismetSystemLibrary.PrintString` "TPS View"))))

(event `Key|LeftMouseButton`
  (params (Key :type "Key Structure"))
  (:`Pressed`
    (bind _asbp_my_player_controller (cast `/MyAssets/Blueprints/BP_MyPlayerController` (`GameplayStatics.GetPlayerController` 0)))
    (if (not (`self.MenuOpened`))
      (`self.Bind Only Once To Left Click` _asbp_my_player_controller (`|CreateDelegate` :!event `SpellLaunch`)))))

(event `Key|Tab`
  (params (Key :type "Key Structure"))
  (:`Pressed`
    (bind _asbp_my_player_controller (cast `/MyAssets/Blueprints/BP_MyPlayerController` (`GameplayStatics.GetPlayerController` 0)))
    (`self.Bind Only Once To Tab` _asbp_my_player_controller (`|CreateDelegate` :!event `Switch View`))))

(event `NewSpell`
  (if (`KismetStringLibrary.EqualEqual_StrStr` "Teleportation" (`/Game/MyAssets/Blueprints/DataAssets/DA_Spell.SpellType` (`self.EquipedSpell`)))
    (`self.Teleportation Spell`)))

(event `Teleportation Spell`
  (bind _asthird_person_character (cast `/Game/ThirdPersonBP/Blueprints/ThirdPersonCharacter` (`GameplayStatics.GetPlayerCharacter` 0)))
  (`KismetSystemLibrary.Delay` 0.5)
  (`self.K2_SetActorLocation` _asthird_person_character (`SceneComponent.RelativeLocation` (`/Game/ThirdPersonBP/Blueprints/ThirdPersonCharacter.SpellSpawner` _asthird_person_character)) false false)
  (`KismetSystemLibrary.PrintString` "Hello"))

(fn `Bind Default`
  (`self.Bind Only Once To E` (`|CreateDelegate` :!event `Bind Default`))
  (`self.Bind Only Once To Left Click` (`|CreateDelegate` :!event `Bind Default`))
  (`self.Bind Only Once To Tab` (`|CreateDelegate` :!event `Bind Default`)))

(fn `Bind Only Once To E`
  (params (Event :type "Delegate (by ref)"))
  (clear `self.OnE`)
  (add `self.OnE` Event))

(fn `Bind Only Once To Left Click`
  (params (Event :type "Delegate (by ref)"))
  (clear `self.OnLeftClick`)
  (add `self.OnLeftClick` Event))

(fn `Bind Only Once To Tab`
  (params (Event :type "Delegate (by ref)"))
  (clear `self.OnTab`)
  (add `self.OnTab` Event))

(fn `UserConstructionScript`)